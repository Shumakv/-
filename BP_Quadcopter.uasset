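; Player-controlled quadcopter pawn with PID-stabilized physics flight driven by four engine components.
; Each tick, throttle shifts a target altitude held by PID, pitch and roll blend input with angle and local-velocity PIDs, and yaw damps angular velocity without input.
; Before takeoff, MoveUp spools RPM for animation and sound until InAir is set.
; Inputs toggle first/third-person cameras and a PID tuning widget, alongside a speedometer HUD.
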(event `self.ReceiveBeginPlay`
  (bind (_returnvalue_x _returnvalue_y _returnvalue_z) (`KismetMathLibrary.BreakVector` (`self.K2_GetActorLocation`)))
  (set `self.DesiredAltitude` _returnvalue_z)
  (bind _asabp_kvad1 (cast `/Game/KVAD1/ABP_KVAD1` (`SkeletalMeshComponent.GetAnimInstance` (`self.KVAD1`))))
  (set `self.As ABP KVAD1` _asabp_kvad1)
  (bind _returnvalue (`|CreateWidget` "/Game/Quadrcopter/UI/PID_Regal.PID_Regal_C"))
  (set `self.Target` _returnvalue)
  (set `/Game/Quadrcopter/UI/PID_Regal.Quadcopter` self _returnvalue)
  (`self.PIDRegal`)
  (`/Game/Quadrcopter/UI/PID_Regal.LoadPID` (`self.Target`))
  (bind _returnvalue_2 (`|CreateWidget` "/Game/Quadrcopter/UI/Speedometr.Speedometr_C" (`GameplayStatics.GetPlayerController` 0)))
  (`UserWidget.AddToViewport` _returnvalue_2 0))

(event `InputAxis|MoveUp`
  (params (AxisValue :type "Float (single-precision)"))
  (bind _rpm (`self.rpm`))
  (bind _kvad1_sound (`self.Kvad1_sound`))
  (bind _as_abp_kvad1 (`self.As ABP KVAD1`))
  (bind _returnvalue (+ (`self.rpm`) (* AxisValue 0.7)))
  (if (not (`self.in air`))
    (set `self.rpm` (`KismetMathLibrary.FClamp` _returnvalue 0.0 51.0))
    (set `self.in air` (> _returnvalue 51.0))
    (`/Engine/EditorBlueprintResources/StandardMacros.IsValid` _as_abp_kvad1
      (:`Is Valid`
        (set `/Game/KVAD1/ABP_KVAD1.rpm` (`self.rpm`) _as_abp_kvad1)
        (`AudioComponent.SetFloatParameter` (`self.Kvad1_sound`) "Pitch" (/ _rpm 100.0))
        (if (> _rpm 10.0)
          (`/Engine/EditorBlueprintResources/StandardMacros.DoOnce` false :!label _label
            (:`Completed`
              (`ActorComponent.Activate` _kvad1_sound false)
              (goto _label_2 :!via `Reset`)))
          (else
            (`/Engine/EditorBlueprintResources/StandardMacros.DoOnce` false :!label _label_2
              (:`Completed`
                (`ActorComponent.Deactivate` _kvad1_sound)
                (goto _label :!via `Reset`)))))))))

(event `self.ReceiveTick`
  (params (DeltaSeconds :type "Float (single-precision)"))
  (`self.HandleThrottle` DeltaSeconds)
  (`self.AltitudeStabilization` DeltaSeconds)
  (`self.HandlePitch` DeltaSeconds)
  (`self.HandleRoll` DeltaSeconds)
  (`self.HandleYaw` DeltaSeconds)
  (`self.CurrentSpeed`))

(event `InputAction|CameraClick`
  (params (Key :type "Key Structure"))
  (:`Pressed`
    (`/Engine/EditorBlueprintResources/StandardMacros.FlipFlop`
      (:`A`
        (`ActorComponent.Activate` (`self.CameraFirst`) false)
        (`ActorComponent.Deactivate` (`self.CameraThird`)))
      (:`B`
        (`ActorComponent.Deactivate` (`self.CameraFirst`))
        (`ActorComponent.Activate` (`self.CameraThird`) false)))))

(event `InputAction|PIDClick`
  (params (Key :type "Key Structure"))
  (bind _target (`self.Target`))
  (:`Pressed`
    (`/Engine/EditorBlueprintResources/StandardMacros.FlipFlop`
      (:`A`
        (`Widget.SetVisibility` _target "Visible"))
      (:`B`
        (`Widget.SetVisibility` _target "Hidden")))))

(fn `AltitudeStabilization`
  (params (DeltaTime :type "Float (double-precision)"))
  (bind (_returnvalue_x _returnvalue_y _returnvalue_z) (`KismetMathLibrary.BreakVector` (`self.K2_GetActorLocation`)))
  (bind _outforce (`/Game/Quadrcopter/BP_Qvad1/BPF_PID.PIDCalculations` _returnvalue_z (`self.DesiredAltitude`) (`self.PAltitude`) (`self.IAltitude`) (`self.DAltitude`) 0.0 DeltaTime (`self.AltitudeIntegral`) (`self.AltitudeErrorPrior`)))
  (for _array_element (`self.EngineArray`)
    (`/Game/Quadrcopter/BP_Qvad1/EngineComponent.AddUpForce` _array_element (* (* _outforce (`self.AltitudeStabilizationForceMultiplier`)) -1.0)))
  (return))

(fn `CurrentSpeed`
  (set `self.CurrentSpeedValue` (`KismetMathLibrary.Conv_IntToDouble` (`KismetMathLibrary.FTrunc` (`KismetMathLibrary.VSize` (`self.GetVelocity` (cast `/BP_Quadcopter` (`GameplayStatics.GetPlayerPawn` 0) :!pure true)))))))

(fn `GetNormalizedRotationPitch`
  (returns (RotationYaw :type "Float (double-precision)"))
  (locals (`Plane Rotation` :type "Float (double-precision)"))
  (bind _output_get (set `local.Plane Rotation` (+ (.pitch (`self.K2_GetActorRotation`)) 45.0)))
  (if (>= _output_get 0.0)
    (return (`KismetMathLibrary.NormalizeToRange` (`local.Plane Rotation`) 0.0 360.0))
    (else
      (return (`KismetMathLibrary.NormalizeToRange` (`local.Plane Rotation`) 0.0 -360.0)))))

(fn `GetNormalizedRotationRoll`
  (returns (RotationYaw :type "Float (double-precision)"))
  (locals (`Plane Rotation` :type "Float (double-precision)"))
  (bind _output_get (set `local.Plane Rotation` (.roll (`self.K2_GetActorRotation`))))
  (if (>= _output_get 0.0)
    (return (`KismetMathLibrary.NormalizeToRange` (`local.Plane Rotation`) 0.0 360.0))
    (else
      (return (`KismetMathLibrary.NormalizeToRange` (`local.Plane Rotation`) 0.0 -360.0)))))

(fn `GetNormalizedRotationYaw`
  (returns (RotationYaw :type "Float (double-precision)"))
  (locals (`Plane Rotation` :type "Float (double-precision)"))
  (bind _output_get (set `local.Plane Rotation` (.yaw (`self.K2_GetActorRotation`))))
  (if (>= _output_get 0.0)
    (return (`KismetMathLibrary.NormalizeToRange` (`local.Plane Rotation`) 0.0 360.0))
    (else
      (return (`KismetMathLibrary.NormalizeToRange` (`local.Plane Rotation`) 0.0 -360.0)))))

(fn `HandlePitch`
  (params (DeltaTime :type "Float (double-precision)"))
  (bind _returnvalue (* (`self.GetInputAxisValue`) (`self.PitchRollMultiplier`)))
  (if (== _returnvalue 0.0)
    (`self.PitchStabilization` DeltaTime)
    (else
      (`self.PitchStabilization` DeltaTime)
      (`self.Pitch` _returnvalue DeltaTime)))
  (return))

(fn `HandleRoll`
  (params (DeltaTime :type "Float (double-precision)"))
  (bind _returnvalue (* (`self.GetInputAxisValue`) (`self.PitchRollMultiplier`)))
  (if (== _returnvalue 0.0)
    (`self.RollStabilization` DeltaTime)
    (else
      (`self.RollStabilization` DeltaTime)
      (`self.Roll` _returnvalue DeltaTime)))
  (return))

(fn `HandleThrottle`
  (params (DeltaTime :type "Float (double-precision)"))
  (set `self.DesiredAltitude` (+ (`self.DesiredAltitude`) (* (* DeltaTime (`self.GetInputAxisValue`)) (`self.ManualThrottleForceMultiplier`)))))

(fn `HandleYaw`
  (params (DeltaTime :type "Float (double-precision)"))
  (bind _returnvalue (* (* (`self.GetInputAxisValue`) 2.0) (`self.YawMultiplier`)))
  (if (== _returnvalue 0.0)
    (`self.YawStabilization` DeltaTime)
    (else
      (`self.Yaw` _returnvalue DeltaTime)))
  (return))

(fn `PIDRegal`
  (bind _returnvalue (`|CreateWidget` "/Game/Quadrcopter/UI/PID_Regal.PID_Regal_C"))
  (set `self.Target` _returnvalue)
  (set `/Game/Quadrcopter/UI/PID_Regal.Quadcopter` self _returnvalue)
  (`UserWidget.AddToViewport` (`self.Target`) 0)
  (set `PlayerController.bShowMouseCursor` true (`GameplayStatics.GetPlayerController` 0))
  (`Widget.SetVisibility` (`self.Target`) "Hidden"))

(fn `Pitch`
  (params (Force :type "Float (double-precision)") (DeltaTime :type "Float (double-precision)"))
  (bind _returnvalue (* Force DeltaTime))
  (if (== _returnvalue 0.0)
    (return)
    (else
      (`/Game/Quadrcopter/BP_Qvad1/EngineComponent.AddUpForce` (`self.Engine1`) _returnvalue)
      (`/Game/Quadrcopter/BP_Qvad1/EngineComponent.AddUpForce` (`self.Engine3`) _returnvalue)
      (bind _result (`/Engine/EditorBlueprintResources/StandardMacros.NegateFloat` _returnvalue)
        (:`  `
          (`/Game/Quadrcopter/BP_Qvad1/EngineComponent.AddUpForce` (`self.Engine2`) _result)
          (`/Game/Quadrcopter/BP_Qvad1/EngineComponent.AddUpForce` (`self.Engine4`) _result)
          (return))))))

(fn `PitchStabilization`
  (params (DeltaTime :type "Float (double-precision)"))
  (bind _box (`self.Box`))
  (bind (_returnvalue_roll _returnvalue_pitch) (`KismetMathLibrary.BreakRotator` (`SceneComponent.K2_GetComponentRotation` (`self.Box`))))
  (bind _returnvalue_x (`KismetMathLibrary.BreakVector` (`KismetMathLibrary.LessLess_VectorRotator` (`SceneComponent.GetComponentVelocity` _box) (`SceneComponent.K2_GetComponentRotation` _box))))
  (bind _outforce (`/Game/Quadrcopter/BP_Qvad1/BPF_PID.PIDCalculations` _returnvalue_pitch 0.0 (`self.PPitch`) (`self.IPitch`) (`self.DPitch`) 0.0 DeltaTime (`self.PitchIntegral`) (`self.PitchErrorPrior`)))
  (bind _outforce_2 (`/Game/Quadrcopter/BP_Qvad1/BPF_PID.PIDCalculations` _returnvalue_x 0.0 (`self.HPitch`) 0.0 0.0 0.0 0.0 (`self.PitchIntegralVelocity`) (`self.PitchErrorPriorVelocity`)))
  (`self.Pitch` (+ (* (* _outforce_2 -1.0) (`self.PitchStabilizationMultiplier`)) (* _outforce (`self.PitchStabilizationMultiplier`))) DeltaTime)
  (return))

(fn `Roll`
  (params (Force :type "Float (double-precision)") (DeltaTime :type "Float (double-precision)"))
  (bind _returnvalue (* Force DeltaTime))
  (if (== _returnvalue 0.0)
    (return)
    (else
      (`/Game/Quadrcopter/BP_Qvad1/EngineComponent.AddUpForce` (`self.Engine1`) _returnvalue)
      (`/Game/Quadrcopter/BP_Qvad1/EngineComponent.AddUpForce` (`self.Engine4`) _returnvalue)
      (bind _result (`/Engine/EditorBlueprintResources/StandardMacros.NegateFloat` _returnvalue)
        (:`  `
          (`/Game/Quadrcopter/BP_Qvad1/EngineComponent.AddUpForce` (`self.Engine2`) _result)
          (`/Game/Quadrcopter/BP_Qvad1/EngineComponent.AddUpForce` (`self.Engine3`) _result)
          (return))))))

(fn `RollStabilization`
  (params (DeltaTime :type "Float (double-precision)"))
  (bind _box (`self.Box`))
  (bind _returnvalue_roll (`KismetMathLibrary.BreakRotator` (`SceneComponent.K2_GetComponentRotation` (`self.Box`))))
  (bind (_returnvalue_x _returnvalue_y) (`KismetMathLibrary.BreakVector` (`KismetMathLibrary.LessLess_VectorRotator` (`SceneComponent.GetComponentVelocity` _box) (`SceneComponent.K2_GetComponentRotation` _box))))
  (bind _outforce (`/Game/Quadrcopter/BP_Qvad1/BPF_PID.PIDCalculations` _returnvalue_roll 0.0 (`self.PRoll`) (`self.IRoll`) (`self.DRoll`) 0.0 DeltaTime (`self.RollIntegral`) (`self.RollErrorPrior`)))
  (bind _outforce_2 (`/Game/Quadrcopter/BP_Qvad1/BPF_PID.PIDCalculations` _returnvalue_y 0.0 (`self.HRoll`) 0.0 0.0 0.0 0.0 (`self.RollIntegralVelocity`) (`self.RollErrorPriorVelocity`)))
  (`self.Roll` (+ (* (* _outforce_2 -1.0) (`self.RollStabilizationMultiplier`)) (* (* _outforce -1.0) (`self.RollStabilizationMultiplier`))) DeltaTime)
  (return))

(fn `UserConstructionScript`
  (`KismetArrayLibrary.Array_Add` (`self.EngineArray`) (`self.Engine1`))
  (`KismetArrayLibrary.Array_Add` (`self.EngineArray`) (`self.Engine2`))
  (`KismetArrayLibrary.Array_Add` (`self.EngineArray`) (`self.Engine3`))
  (`KismetArrayLibrary.Array_Add` (`self.EngineArray`) (`self.Engine4`)))

(fn `Yaw`
  (params (Force :type "Float (double-precision)") (DeltaTime :type "Float (double-precision)"))
  (bind _returnvalue (* Force DeltaTime))
  (if (== _returnvalue 0.0)
    (return)
    (else
      (for _array_element (`self.EngineArray`)
        (`/Game/Quadrcopter/BP_Qvad1/EngineComponent.AddYawForce` _array_element _returnvalue)
        (return))
      (return))))

(fn `YawStabilization`
  (params (DeltaTime :type "Float (double-precision)"))
  (bind (_returnvalue_x _returnvalue_y _returnvalue_z) (`KismetMathLibrary.BreakVector` (`PrimitiveComponent.GetPhysicsAngularVelocityInDegrees` (`self.Box`) "None")))
  (bind _outforce (`/Game/Quadrcopter/BP_Qvad1/BPF_PID.PIDCalculations` _returnvalue_z 0.0 (`self.PYaw`) (`self.IYaw`) (`self.DYaw`) 0.0 DeltaTime (`self.YawIntegral`) (`self.YawErrorPrior`)))
  (`self.Yaw` (* (* _outforce -1.0) (`self.YawStabilizationMultiplier`)) DeltaTime)
  (return))